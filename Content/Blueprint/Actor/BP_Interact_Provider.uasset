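; BP_Interact_Provider is an interactable actor that updates the quest system of whoever interacts with it.
; Its CanInteract event runs the parent logic, then looks up BPC_QuestSystem on the instigator.
; If that component is valid, it calls UpdateQuestSystem with the quest gameplay tag as origin and the updated gameplay tag as collected.
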(event `/Game/Blueprint/Interface/BPI_Interaction.CanInteract`
  (params (Instigator :type "/Game/ThirdPerson/Blueprints/BP_ThirdPersonCharacter Object Reference"))
  (bind _returnvalue (`self.GetComponentByClass` Instigator "/Game/Blueprint/Component/BPC_QuestSystem.BPC_QuestSystem_C"))
  (`parent.CanInteract` Instigator)
  (`/Engine/EditorBlueprintResources/StandardMacros.IsValid` _returnvalue
    (:`Is Valid`
      (`/Game/Blueprint/Component/BPC_QuestSystem.UpdateQuestSystem` _returnvalue (`self.QuestGameplayTag`) (`self.UpdatedGameplayTag`)))))

(fn `UserConstructionScript`
  (`parent.UserConstructionScript`))