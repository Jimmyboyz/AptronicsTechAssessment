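; Quest component that tracks current and finished quests as gameplay tag containers and prints feedback as debug text.
; AddQuestSystem uses the quest tag as a DT_QuestData row name and adds the quest once its prerequisite quests are finished.
; UpdateQuestSystem increments per-tag counts in a map, then CheckingQuestSystem compares them to the row's completion requirements.
; Completed quests move to the finished container and their counters are cleared.
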(event `AddQuestSystem`
  (params (NewQuestTag :type "GameplayTag Structure"))
  (bind _finishedquestcontainer_gameplaytags (break `GameplayTagContainer` (`self.FinishedQuestContainer`)))
  (if (not (`BlueprintGameplayTagLibrary.HasTag` (`self.FinishedQuestContainer`) NewQuestTag))
    (bind _returnvalue (`|GetDataTableRow` "/Game/DataTable/DT_QuestData.DT_QuestData" (`BlueprintGameplayTagLibrary.GetTagName` NewQuestTag))
      (:`then`
        (bind _requiredmainquest_gameplaytags (break `GameplayTagContainer` (break `QuestData` _returnvalue)))
        (if (> (`KismetArrayLibrary.Array_Length` _requiredmainquest_gameplaytags) 0)
          (set `self.bHasRequiredQuest` false)
          (for _array_element _requiredmainquest_gameplaytags :!label _label
            (if (`KismetArrayLibrary.Array_Contains` _finishedquestcontainer_gameplaytags _array_element)
              (set `self.bHasRequiredQuest` true)
              (else
                (set `self.bHasRequiredQuest` false)
                (`self.BreakCheckingHasRequiredQuest`))))
          (if (`self.bHasRequiredQuest`)
            (if (not (`BlueprintGameplayTagLibrary.HasTag` (`self.CurrentQuestContainer`) NewQuestTag true)) :!label _label_2
              (`BlueprintGameplayTagLibrary.AddGameplayTag` (`self.CurrentQuestContainer`) NewQuestTag)
              (`KismetSystemLibrary.PrintText` (`|FormatText` "Quest {0} Is added in your quest list." (`.RightS` (`KismetStringLibrary.Split` (`KismetStringLibrary.Conv_NameToString` (`BlueprintGameplayTagLibrary.GetTagName` NewQuestTag)) "." "IgnoreCase" "FromEnd"))) true true (struct :`R` 0.5 :`G` 0.5 :`A` 1.0) 10.0)
              (else
                (`KismetSystemLibrary.PrintText` (`|FormatText` "Quest {0} Is already in your quest list." (`.RightS` (`KismetStringLibrary.Split` (`KismetStringLibrary.Conv_NameToString` (`BlueprintGameplayTagLibrary.GetTagName` NewQuestTag)) "." "IgnoreCase" "FromEnd"))))))
            (else
              (`KismetSystemLibrary.PrintText` (`|FormatText` "Quest {0} need to finish before proceed to this quest." (`.RightS` (`KismetStringLibrary.Split` (`KismetStringLibrary.Conv_NameToString` (`BlueprintGameplayTagLibrary.GetTagName` _array_element)) "." "IgnoreCase" "FromEnd"))))))
          (else
            (goto _label_2)))))
    (else
      (`KismetSystemLibrary.PrintText` (`|FormatText` "Quest {0} is finished." (`.RightS` (`KismetStringLibrary.Split` (`KismetStringLibrary.Conv_NameToString` (`BlueprintGameplayTagLibrary.GetTagName` NewQuestTag)) "." "IgnoreCase" "FromEnd")))))))

(event `BreakCheckingHasRequiredQuest`
  (goto _label :!via `Break`))

(event `UpdateQuestSystem`
  (params (OriginQuestTag :type "GameplayTag Structure") (CollectedQuestTag :type "GameplayTag Structure"))
  (bind _collectedquestarray (`self.CollectedQuestArray`))
  (if (`BlueprintGameplayTagLibrary.HasTag` (`self.CurrentQuestContainer`) OriginQuestTag)
    (if (`BlueprintMapLibrary.Map_Contains` _collectedquestarray CollectedQuestTag)
      (bind _result (`/Engine/EditorBlueprintResources/StandardMacros.IncrementInt` (`BlueprintMapLibrary.Map_Find` _collectedquestarray CollectedQuestTag))
        (:`  `
          (`BlueprintMapLibrary.Map_Add` _collectedquestarray CollectedQuestTag _result)
          (`self.CheckingQuestSystem` OriginQuestTag)))
      (else
        (`BlueprintMapLibrary.Map_Add` (`self.CollectedQuestArray`) CollectedQuestTag 1)
        (`self.CheckingQuestSystem` OriginQuestTag)))))

(event `CheckingQuestSystem`
  (params (OriginQuestTag :type "GameplayTag Structure"))
  (bind _returnvalue (`|GetDataTableRow` "/Game/DataTable/DT_QuestData.DT_QuestData" (`BlueprintGameplayTagLibrary.GetTagName` OriginQuestTag))
    (:`then`
      (bind ((`RequiredMainQuest` _requiredmainquest) (`RequiredCompletionDetails` _requiredcompletiondetails)) (break `QuestData` _returnvalue))
      (bind _keys (`BlueprintMapLibrary.Map_Keys` _requiredcompletiondetails))
      (for _array_element _keys :!label _label_3
        (bind (_value _returnvalue_2) (`BlueprintMapLibrary.Map_Find` (`self.CollectedQuestArray`) _array_element))
        (if _returnvalue_2
          (if (>= _value (`BlueprintMapLibrary.Map_Find` _requiredcompletiondetails _array_element))
            (set `self.bIsQuestDone` true)
            (else
              (set `self.bIsQuestDone` false :!label _label_4)
              (`self.StopCheckingQuest`)))
          (else
            (goto _label_4))))
      (if (`self.bIsQuestDone`)
        (`|ExecutionSequence`
          (:`then_0`
            (`BlueprintGameplayTagLibrary.AddGameplayTag` (`self.FinishedQuestContainer`) OriginQuestTag))
          (:`then_1`
            (`BlueprintGameplayTagLibrary.RemoveGameplayTag` (`self.CurrentQuestContainer`) OriginQuestTag))
          (:`then_2`
            (bind _keys_2 (`BlueprintMapLibrary.Map_Keys` _requiredcompletiondetails))
            (for _array_element_2 _keys_2
              (`BlueprintMapLibrary.Map_Remove` (`self.CollectedQuestArray`) _array_element_2)))
          (:`then_3`
            (`KismetSystemLibrary.PrintText` (`|FormatText` "You have completed Quest {0}!" (`.RightS` (`KismetStringLibrary.Split` (`KismetStringLibrary.Conv_NameToString` (`BlueprintGameplayTagLibrary.GetTagName` OriginQuestTag)) "." "IgnoreCase" "FromEnd"))) true true (struct :`G` 1.0 :`A` 1.0) 10.0)))))))

(event `StopCheckingQuest`
  (goto _label_3 :!via `Break`))